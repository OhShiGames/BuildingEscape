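; An openable door actor that swings open and closed in response to its OpenDoor OnOpen and OnClose events.
; The OpenDoorSwing timeline plays on open and reverses on close, adding its OpenAngle yaw to the rotation cached at BeginPlay.
; A Sound Timing event track on the timeline plays the Doorlock sound at the door's location.
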(event `self.ReceiveBeginPlay`
  (set `self.Initial Rotation` (`self.K2_GetActorRotation`)))

(event `self.OpenDoor.OnOpen`
  (bind (_direction _open_angle) (`Timeline|Open Door Swing` :!label _label)
    (:`Update`
      (`self.SetActorRotation` (`KismetMathLibrary.ComposeRotators` (`KismetMathLibrary.MakeRotator` 0.0 0.0 _open_angle) (`self.Initial Rotation`))))
    (:`Sound Timing`
      (`GameplayStatics.PlaySoundAtLocation` "/Game/Audio/door-lock.door-lock" (`self.K2_GetActorLocation`) (struct) 0.5))))

(event `self.OpenDoor.OnClose`
  (goto _label :!via `Reverse`))

(fn `UserConstructionScript`)